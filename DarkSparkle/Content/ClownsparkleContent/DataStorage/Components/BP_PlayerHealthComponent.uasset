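; Player health component that keeps its health value in the game instance's player stats.
; On BeginPlay it loads Health from those stats before running the parent's BeginPlay.
; It extends the parent's Heal and TakeDamage, writing the resulting Health back to the game instance after each call.
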(event EventBeginPlay
  (bind _asbp_game_instance (Utilities|Casting|CastToBP_GameInstance (Game|GetGameInstance)))
  (Variables|Default|SetGameInstanceRef _asbp_game_instance)
  (Variables|Default|SetHealth (.Health (Utilities|Struct|BreakPlayerInformation (Variables|/Game/ClownsparkleContent/Blueprints/BP_GameInstance.BP_GameInstance_C|GetPlayerStats (Variables|Default|GetGameInstanceRef)))))
  (|CallParentFunction))

(event EventTick
  (params (DeltaSeconds :type Float%20%28single-precision%29))
  (|CallParentFunction DeltaSeconds) ; This node is disabled and will not be called.\nDrag off pins to build functionality.
)

(fn Heal
  (params (HealAmt :type Integer))
  (|CallParentFunction HealAmt)
  (Utilities|Struct|SetmembersinPlayerInformation (Variables|/Game/ClownsparkleContent/Blueprints/BP_GameInstance.BP_GameInstance_C|GetPlayerStats (Variables|Default|GetGameInstanceRef)) (Variables|Default|GetHealth)))

(fn TakeDamage
  (params (DamageAmt :type Integer))
  (|CallParentFunction DamageAmt)
  (Utilities|Struct|SetmembersinPlayerInformation (Variables|/Game/ClownsparkleContent/Blueprints/BP_GameInstance.BP_GameInstance_C|GetPlayerStats (Variables|Default|GetGameInstanceRef)) (Variables|Default|GetHealth)))