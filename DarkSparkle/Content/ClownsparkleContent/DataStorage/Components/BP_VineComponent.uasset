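; BP_VineComponent is an actor component that removes its owning actor, presumably a vine, based on the deer species' status in the biodiversity data.
; On BeginPlay it reads the deer criteria from BP_GameInstance's BiodiversityStats and destroys the owner if the status matches the enum's NewEnumerator0 entry.
; The check runs only once, as Tick is disabled.
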(event EventBeginPlay
  (bind _asbp_game_instance (Utilities|Casting|CastToBP_GameInstance (Game|GetGameInstance)))
  (Variables|Default|SetAs%20BP%20Game%20Instance _asbp_game_instance)
  (if (Utilities|Enum|Equal(Enum) (Utilities|Struct|BreakEnemyComponent (Utilities|Struct|BreakBiodiversityComponents (Variables|/Game/ClownsparkleContent/Blueprints/BP_GameInstance.BP_GameInstance_C|GetBiodiversityStats (Variables|Default|GetAs%20BP%20Game%20Instance)))) "NewEnumerator0")
    (Actor|DestroyActor (Components|GetOwner))))

(event EventTick
  (params (DeltaSeconds :type Float%20%28single-precision%29)))