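; BP_HealthComponent is a health component that tracks health and signals when it runs out.
; It caps Health at MaxHealth on BeginPlay and when healing, and floors it at zero when taking damage.
; TakeDamage calls the OnDeath dispatcher whenever the resulting health is zero, including on repeated hits after death.
; The Death function is an empty stub, and Tick does nothing.
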(event EventBeginPlay
  (Variables|Default|SetHealth (Math|Integer|Min(Integer) (Variables|Default|GetHealth) (Variables|Default|GetMaxHealth))))

(event EventTick
  (params (DeltaSeconds :type Float%20%28single-precision%29)))

(fn TakeDamage
  (params (DamageAmt :type Integer))
  (Variables|Default|SetHealth (Math|Integer|Max(Integer) (- (Variables|Default|GetHealth) DamageAmt)))
  (if (<= (Variables|Default|GetHealth) 0)
    (Default|CallOnDeath)))

(fn Heal
  (params (HealAmt :type Integer))
  (Variables|Default|SetHealth (Math|Integer|Min(Integer) (+ HealAmt (Variables|Default|GetHealth)) (Variables|Default|GetMaxHealth))))

(fn Death)