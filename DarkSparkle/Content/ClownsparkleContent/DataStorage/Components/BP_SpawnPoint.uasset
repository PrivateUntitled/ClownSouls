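; BP_SpawnPoint is a component that spawns an enemy at its owner's transform when play begins.
; It switches on EnemyToSpawn: Regular spawns BP_BaseEnemy, while Boss spawns BP_BaseBoss only if the SampleBossToSpawn flag in the game instance's SpecialEnemySpawn data is set.
; Both paths require a successful cast to BP_GameInstance, and no Tick logic runs.
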(event EventBeginPlay
  (bind _returnvalue (Components|GetOwner))
  (bind _returnvalue_2 (Transformation|GetActorTransform _returnvalue))
  (bind _asbp_game_instance (Utilities|Casting|CastToBP_GameInstance (Game|GetGameInstance)))
  (switch Utilities|FlowControl|Switch|SwitchonEnemyTypes (Variables|Default|GetEnemyToSpawn)
    (:NewEnumerator0
      (Game|SpawnActorfromClass "/Game/ClownsparkleContent/Blueprints/Characters/BasicEnemies/BP_BaseEnemy.BP_BaseEnemy_C" _returnvalue_2 "Undefined" "MultiplyWithRoot" 0 0))
    (:NewEnumerator1
      (if (Utilities|Struct|BreakSpecialEnemyStruct (Variables|/Game/ClownsparkleContent/Blueprints/BP_GameInstance.BP_GameInstance_C|GetSpecialEnemySpawn _asbp_game_instance))
        (Game|SpawnActorfromClass "/Game/ClownsparkleContent/Blueprints/Characters/Bosses/BP_BaseBoss.BP_BaseBoss_C" _returnvalue_2 "Undefined" "MultiplyWithRoot" 0 0)))))

(event EventTick
  (params (DeltaSeconds :type Float%20%28single-precision%29)))