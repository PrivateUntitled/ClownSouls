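; Harvestable component that holds a list of item drops and tallies them against the player's loot stored in BP_GameInstance.
; It caches the game instance on BeginPlay.
; AddToPlayerLoot switches on each drop's item type to copy the matching PlayerLoot entry into DropToAdd, then adds the amount and prints the total.
; The updated total is set on DropToAdd, with no explicit write back to PlayerLoot.
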(event EventBeginPlay
  (bind _asbp_game_instance (Utilities|Casting|CastToBP_GameInstance (Game|GetGameInstance)))
  (Variables|Default|SetGameInstanceRef _asbp_game_instance))

(event EventTick
  (params (DeltaSeconds :type Float%20%28single-precision%29)))

(fn AddtoPlayerLoot
  (bind _gameinstanceref (Variables|Default|GetGameInstanceRef))
  (bind _playerloot (Variables|/Game/ClownsparkleContent/Blueprints/BP_GameInstance.BP_GameInstance_C|GetPlayerLoot _gameinstanceref))
  (for _array_element (Variables|Default|GetDrops)
    (Utilities|FlowControl|Sequence
      (:then_0
        (switch Utilities|FlowControl|Switch|SwitchonLoot (.item _array_element)
          (:NewEnumerator0
            (LocalVariables|SetDropToAdd (Variables|/Game/ClownsparkleContent/DataStorage/DataAssets/PlayerData/PDA_PlayerLoot.PDA_PlayerLoot_C|GetSunSlimeEssence _playerloot)))
          (:NewEnumerator1
            (LocalVariables|SetDropToAdd (Variables|/Game/ClownsparkleContent/DataStorage/DataAssets/PlayerData/PDA_PlayerLoot.PDA_PlayerLoot_C|GetAntlerShard _playerloot)))
          (:NewEnumerator2
            (LocalVariables|SetDropToAdd (Variables|/Game/ClownsparkleContent/DataStorage/DataAssets/PlayerData/PDA_PlayerLoot.PDA_PlayerLoot_C|GetDeerFoot _playerloot)))
          (:NewEnumerator3
            (LocalVariables|SetDropToAdd (Variables|/Game/ClownsparkleContent/DataStorage/DataAssets/PlayerData/PDA_PlayerLoot.PDA_PlayerLoot_C|GetRoseEssence _playerloot)))
          (:NewEnumerator4
            (LocalVariables|SetDropToAdd (Variables|/Game/ClownsparkleContent/DataStorage/DataAssets/PlayerData/PDA_PlayerLoot.PDA_PlayerLoot_C|GetRoseThorns _playerloot)))
          (:NewEnumerator5
            (LocalVariables|SetDropToAdd (Variables|/Game/ClownsparkleContent/DataStorage/DataAssets/PlayerData/PDA_PlayerLoot.PDA_PlayerLoot_C|GetWolfEssence _playerloot)))
          (:NewEnumerator7
            (LocalVariables|SetDropToAdd (Variables|/Game/ClownsparkleContent/DataStorage/DataAssets/PlayerData/PDA_PlayerLoot.PDA_PlayerLoot_C|GetBatWings _playerloot)))
          (:NewEnumerator8
            (LocalVariables|SetDropToAdd (Variables|/Game/ClownsparkleContent/DataStorage/DataAssets/PlayerData/PDA_PlayerLoot.PDA_PlayerLoot_C|GetFur _playerloot)))
          (:NewEnumerator9
            (LocalVariables|SetDropToAdd (Variables|/Game/ClownsparkleContent/DataStorage/DataAssets/PlayerData/PDA_PlayerLoot.PDA_PlayerLoot_C|GetTwig _playerloot)))
          (:NewEnumerator10
            (LocalVariables|SetDropToAdd (Variables|/Game/ClownsparkleContent/DataStorage/DataAssets/PlayerData/PDA_PlayerLoot.PDA_PlayerLoot_C|GetStone _playerloot)))))
      (:then_1
        (Utilities|Struct|SetmembersinDropAmount (LocalVariables|GetDropToAdd) (+ (Utilities|Struct|BreakDropAmount (LocalVariables|GetDropToAdd)) (.amount _array_element)))
        (Development|PrintString (Utilities|String|ToString(Text) (Utilities|Text|FormatText "{0} {1}" (Utilities|String|EnumtoString (.item _array_element)) (Utilities|Struct|BreakDropAmount (LocalVariables|GetDropToAdd)))))))))