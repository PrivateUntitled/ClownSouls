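; BP_SwordTrail is an animation notify state that drives a sword trail effect during an animation.
; On each notify tick it gets the spawned effect for the mesh and feeds the world locations of its start and end sockets into the matching vector parameters.
; If no valid effect exists, it prints a debug failure message and returns false.
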(fn ReceivedNotifyTick
  (params (MeshComp :type Skeletal%20Mesh%20Component%20Object%20Reference) (Animation :type Anim%20Sequence%20Base%20Object%20Reference) (FrameDeltaTime :type Float%20%28single-precision%29) (EventReference :type Anim%20Notify%20Event%20Reference%20Structure%20%28by%20ref%29))
  (bind _returnvalue (Class|AnimNotifyStateTimedNiagaraEffect|GetSpawnedEffect MeshComp))
  (Utilities|IsValid _returnvalue
    (:Is%20Valid
      (Effects|Components|ParticleSystem|SetVectorParameter _returnvalue "StartSocket" (Transformation|GetSocketLocation MeshComp (Variables|Default|GetStartSocket)))
      (Effects|Components|ParticleSystem|SetVectorParameter _returnvalue "EndSocket" (Transformation|GetSocketLocation MeshComp (Variables|Default|GetEndSocket)))
      (return true))
    (:Is%20Not%20Valid
      (Development|PrintString 0 "ITS NOT WORKING")
      (return false))))