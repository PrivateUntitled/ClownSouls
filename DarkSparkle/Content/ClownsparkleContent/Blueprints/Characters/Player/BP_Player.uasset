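; Player character Blueprint that carries a sword and shield, tracks health and hunger, and handles climb, dodge and block actions.
; BeginPlay attaches weapons to mesh sockets, loads health from the game instance, starts a looping hunger timer and binds action events.
; Actions switch between character and climbing movement components or change speed.
; Tick locks camera and body rotation onto any targeted enemy, while heavy attack logic sits archived and unwired.
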(event Custom|DoClimb
  (params (ActionStates :type ActionStates%20Enum :default "NewEnumerator0") (WallRef :type BP%20Climable%20Wall%20Object%20Reference))
  (switch Utilities|FlowControl|Switch|SwitchonActionStates ActionStates
    (:NewEnumerator0
      (CallFunction|SetMovementCompoment true)
      (Variables|References|SetClimableWallRef WallRef))
    (:NewEnumerator1
      (CallFunction|SetMovementCompoment false)
      (Variables|References|SetClimableWallRef 0))))

(event Custom|DoDodge
  (params (Action%20States :type ActionStates%20Enum :default "NewEnumerator0"))
  (switch Utilities|FlowControl|Switch|SwitchonActionStates Action%20States
    (:NewEnumerator0
      (CallFunction|SetMovementCompoment true)
      (CallFunction|SetPlayerSpeed (Variables|Speed|GetDodgeSpeed)))
    (:NewEnumerator1
      (CallFunction|SetMovementCompoment false)
      (CallFunction|SetPlayerSpeed (Variables|Speed|GetNormalSpeed)))))

(event Custom|DoHeavyAttack
  ;[1 0.1198 0.1198] Archived - Heavy Attack
)

(event Custom|ChargeHeavy
  ;[1 0.1198 0.1198] Archived - Heavy Attack
)

(event Custom|HoldCharge
  (bind _playeranimref (Variables|References|GetPlayerAnimRef))
  ;[1 0.1198 0.1198] Archived - Heavy Attack
  (Variables|/Game/ClownsparkleContent/Assets/PlaceHolderAssets/Character/AB_Player.AB_Player_C|SetChargingAnim _playeranimref false)
  (Variables|/Game/ClownsparkleContent/Assets/PlaceHolderAssets/Character/AB_Player.AB_Player_C|SetHoldChargeAnim _playeranimref false))

(event Custom|TakeDamage
  (params (DamageTaken :type Integer))
  (Default|TakeDamage (Variables|Default|GetBP_HealthComponent) DamageTaken))

(event Custom|DoBlock
  (params (ActionStates :type ActionStates%20Enum :default "NewEnumerator0"))
  (switch Utilities|FlowControl|Switch|SwitchonActionStates ActionStates
    (:NewEnumerator0
      (CallFunction|SetPlayerSpeed (Variables|Speed|GetBlockSpeed)))
    (:NewEnumerator1
      (CallFunction|SetPlayerSpeed (Variables|Speed|GetNormalSpeed)))))

(event EventTick
  (params (DeltaSeconds :type Float%20%28single-precision%29))
  (bind _targettedenemy (Variables|References|GetTargettedEnemy))
  (bind _capsulecomponent (Variables|Collision|GetCapsuleComponent))
  (bind _returnvalue (Transformation|GetWorldLocation _capsulecomponent))
  (bind _targetpoint (Variables|/Game/ClownsparkleContent/Blueprints/Characters/Enemies/BaseEnemy/BP_BaseEnemy.BP_BaseEnemy_C|GetTargetPoint _targettedenemy))
  (bind _returnvalue_2 (Transformation|GetWorldLocation _targetpoint))
  (bind _returnvalue_3 (Math|Rotator|FindLookatRotation _returnvalue _returnvalue_2))
  (bind (_roll _pitch _yaw) (Math|Rotator|BreakRotator _returnvalue_3))
  (if (!= (Variables|References|GetTargettedEnemy) 0)
    ;[1 1 1] Rotate Camera facing the Enemy
    (Pawn|SetControlRotation (Pawn|GetController) _returnvalue_3)
    ;[1 1 1] Rotate Body Facing Enemy
    (Transformation|SetWorldRotation (Variables|Collision|GetCapsuleComponent) (Math|Rotator|MakeRotator _roll 0.0 _yaw) true false)))

(event EventBeginPlay
  (bind _mesh (Variables|Character|GetMesh))
  (bind _mesh_2 (Variables|Character|GetMesh))
  (Utilities|FlowControl|Sequence
    (:then_0
      ;[0.1927 0.1927 0.1927] Equip Sword to Left Hand
      (bind _returnvalue (Game|SpawnActorfromClass "/Game/ClownsparkleContent/Blueprints/Actors/PlayerTools/BP_Sword.BP_Sword_C" (Math|Transform|MakeTransform "0, 0, 0" "0, 0, 0" "1.000000,1.000000,1.000000") "Undefined" "MultiplyWithRoot" 0 0))
      (Transformation|AttachComponentToComponent _returnvalue _mesh (Variables|/Script/Engine.SkeletalMeshSocket|GetSocketName (Class|SkeletalMesh|GetSocketbyIndex (Variables|/Script/Engine.SkeletalMeshComponent|GetSkeletalMeshAsset _mesh) 1)) "SnapToTarget" "SnapToTarget" "SnapToTarget" true)
      ;[1 1 1] Equip Shield at the Right Hand
      (bind _returnvalue_2 (Game|SpawnActorfromClass "/Game/ClownsparkleContent/Blueprints/Actors/PlayerTools/BP_Shield.BP_Shield_C" (Math|Transform|MakeTransform "0, 0, 0" "0, 0, 0" "1.000000,1.000000,1.000000") "Undefined" "MultiplyWithRoot" 0 0))
      (Transformation|AttachComponentToComponent _returnvalue_2 _mesh_2 (Variables|/Script/Engine.SkeletalMeshSocket|GetSocketName (Class|SkeletalMesh|GetSocketbyIndex (Variables|/Script/Engine.SkeletalMeshComponent|GetSkeletalMeshAsset _mesh_2))) "SnapToTarget" "SnapToTarget" "SnapToTarget" true)
      (Variables|References|SetShield _returnvalue_2))
    (:then_1
      (bind _asab_player (Utilities|Casting|CastToAB_Player (Components|SkeletalMesh|GetAnimInstance (Variables|Character|GetMesh))))
      (Variables|References|SetPlayerAnimRef _asab_player))
    (:then_2
      ;[1 1 1] Make Player Hungrier
      (Utilities|Time|SetTimerbyEvent (EventDispatchers|CreateEvent :!event LoseHunger) (Variables|HungerStats|GetHungerDuration) true))
    (:then_3
      (bind _asbp_game_instance (Utilities|Casting|CastToBP_GameInstance (Game|GetGameInstance)))
      (Variables|/Game/ClownsparkleContent/DataStorage/Components/BP_HealthComponent.BP_HealthComponent_C|SetHealth (Variables|Default|GetBP_HealthComponent) (Utilities|Struct|BreakPlayerInformation (Variables|/Game/ClownsparkleContent/Blueprints/BP_GameInstance.BP_GameInstance_C|GetPlayerStats _asbp_game_instance)))
      (EventDispatchers|BindEventtoAttacked (EventDispatchers|CreateEvent :!event Custom|TakeDamage))
      (EventDispatchers|BindEventtoBlock (EventDispatchers|CreateEvent :!event Custom|DoBlock))
      (EventDispatchers|BindEventtoClimb (EventDispatchers|CreateEvent :!event Custom|DoClimb))
      (EventDispatchers|BindEventtoDodge (EventDispatchers|CreateEvent :!event Custom|DoDodge))
      (Default|CallClimb "NewEnumerator1"))))

(fn ConstructionScript)

(fn LoseHunger
  (Variables|HungerStats|SetHunger (- (Variables|HungerStats|GetHunger) (Variables|HeavyAttack|GetHungerLoss))))

(fn SetMovementCompoment
  (params (DeactivateCharacterMovement? :type Boolean))
  (if DeactivateCharacterMovement?
    (Components|Activation|Deactivate (Variables|Character|GetCharacterMovement))
    (Components|Activation|Activate (Variables|Default|GetCharacter%20Climbing%20) false)
    (else
      (Components|Activation|Deactivate (Variables|Default|GetCharacter%20Climbing%20))
      (Components|Activation|Activate (Variables|Character|GetCharacterMovement) false))))

(fn SetPlayerSpeed
  (params (Speed :type Float%20%28double-precision%29))
  (Utilities|FlowControl|Sequence
    (:then_0
      (Variables|/Script/Engine.CharacterMovementComponent|SetMaxWalkSpeed (Variables|Character|GetCharacterMovement) Speed))
    (:then_1
      (Variables|/Script/Engine.FloatingPawnMovement|SetMaxSpeed (Variables|Default|GetCharacter%20Climbing%20) Speed))))

(fn PlayerSpeed)