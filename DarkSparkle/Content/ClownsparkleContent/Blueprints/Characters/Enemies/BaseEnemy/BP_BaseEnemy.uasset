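; Base enemy character, configured by MonsterInfo, that fights the player and drops loot on death.
; Taking damage switches its AI controller to attack phase, raises speed, reduces health and sets invincibility, which a light-attack-style event updates.
; Attacks line-trace between player and enemy so a shield absorbs damage.
; Death flags the blackboard, spawns weighted-chance loot and fades dynamic materials before destroying the actor.
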(event Custom|Die
  (bind _enemycontrollerref (Variables|Default|GetEnemyControllerRef))
  (Utilities|FlowControl|Sequence
    (:then_0
      ;[1 1 1] Turn HP Bar Invisible
      (Rendering|SetVisibility (Variables|Default|GetWidget) false false))
    (:then_1
      ;[1 1 1] Disable Collissions
      (Collision|SetCollisionEnabled (Variables|Collision|GetCapsuleComponent) "NoCollision")
      (Collision|SetCollisionEnabled (Variables|Character|GetMesh) "NoCollision"))
    (:then_2
      ;[1 1 1] Drop Monster Loot
      (CallFunction|DropLoot)
      (AI|Components|Blackboard|SetValueasBool (Variables|/Script/AIModule.AIController|GetBlackboard _enemycontrollerref) (Variables|/Game/ClownsparkleContent/Blueprints/Characters/Enemies/BaseEnemy/BP_BaseEnemyController.BP_BaseEnemyController_C|GetIsDeadTag _enemycontrollerref) true))
    (:then_3
      ;[1 1 1] Fade Out Animation - Material
      (bind _opacity (Timeline|Timeline Play)
        (:Update
          (for (_ _array_index) (Rendering|Material|GetMaterials (Variables|Character|GetMesh))
            (Rendering|Material|SetMaterial (Variables|Character|GetMesh) _array_index (Variables|Default|GetDeathMaterial))
            (bind _returnvalue (Rendering|Material|CreateDynamicMaterialInstance (Variables|Character|GetMesh) _array_index (Rendering|Material|GetMaterial (Variables|Character|GetMesh) _array_index) "None" :!class /Script/Engine.PrimitiveComponent))
            (Rendering|Material|SetScalarParameterValue _returnvalue "Opacity" _opacity :!class /Script/Engine.MaterialInstanceDynamic)))
        (:Finished
          (Actor|DestroyActor))))))

(event Custom|TakeDamage
  (params (TotalDamage :type Integer))
  (Utilities|FlowControl|Sequence
    (:then_0
      ;[1 1 1] Make Enemies Attack
      (Default|SetAttackPhase (Variables|Default|GetEnemyControllerRef))
      (CallFunction|SetSpeed (Variables|/Game/ClownsparkleContent/DataStorage/DataAssets/Monsters/PDA_MonsterInformation.PDA_MonsterInformation_C|GetAttackMoveSpeed (Variables|Default|GetMonsterInfo))))
    (:then_1
      ;[1 1 1] Take Damage
      (Default|TakeDamage (Variables|Default|GetBP_HealthComponent) TotalDamage))
    (:then_2
      ;[1 1 1] Set Invincibility
      (Variables|Default|SetInvincible true))))

(event Custom|CustomEvent_0
  (params (NewParam :type AttackStages%20Enum :default "NewEnumerator0"))
  (Variables|Default|SetInvincible (Utilities|Enum|Equal(Enum) NewParam "NewEnumerator2")))

(event EventBeginPlay
  (bind _bp_healthcomponent (Variables|Default|GetBP_HealthComponent))
  (Utilities|FlowControl|Sequence
    (:then_0
      ;[1 1 1] Setting References
      (bind _asbp_player (Utilities|Casting|CastToBP_Player (Game|Player|GetPlayerPawn 0)))
      (Variables|Default|SetPlayerRef _asbp_player)
      (bind _asbp_base_enemy_controller (Utilities|Casting|CastToBP_BaseEnemyController (Pawn|GetController)))
      (Variables|Default|SetEnemyControllerRef _asbp_base_enemy_controller)
      (bind _asbp_enemy_ui (Utilities|Casting|CastToBP_EnemyUI (UserInterface|GetWidget (Variables|Default|GetWidget))))
      (Default|SetEnemyRef _asbp_enemy_ui self))
    (:then_1
      ;[1 1 1] Player Camera Ignores Enemy Collision
      (Collision|SetCollisionResponsetoChannel (Variables|Character|GetMesh) "ECC_Camera" "ECR_Ignore"))
    (:then_2
      (CallFunction|SetSpeed (Variables|/Game/ClownsparkleContent/DataStorage/DataAssets/Monsters/PDA_MonsterInformation.PDA_MonsterInformation_C|GetWanderMoveSpeed (Variables|Default|GetMonsterInfo)))
      (Variables|/Game/ClownsparkleContent/DataStorage/Components/BP_HealthComponent.BP_HealthComponent_C|SetHealth _bp_healthcomponent (Variables|/Game/ClownsparkleContent/DataStorage/DataAssets/Monsters/PDA_MonsterInformation.PDA_MonsterInformation_C|GetHealth (Variables|Default|GetMonsterInfo)))
      (Variables|/Game/ClownsparkleContent/DataStorage/Components/BP_HealthComponent.BP_HealthComponent_C|SetMaxHealth _bp_healthcomponent (Variables|/Game/ClownsparkleContent/DataStorage/DataAssets/Monsters/PDA_MonsterInformation.PDA_MonsterInformation_C|GetHealth (Variables|Default|GetMonsterInfo))))
    (:then_3
      ;[1 1 1] Binding Events
      (EventDispatchers|BindEventtoOnDeath (Variables|Default|GetBP_HealthComponent) (EventDispatchers|CreateEvent :!event Custom|Die))
      (EventDispatchers|BindEventtoAttacked (EventDispatchers|CreateEvent :!event Custom|TakeDamage))
      (EventDispatchers|BindEventtoLightAttack (Variables|Default|GetPlayerRef) (EventDispatchers|CreateEvent :!event Custom|CustomEvent_0))
      (AI|Components|Blackboard|SetValueasBool (Variables|/Script/AIModule.AIController|GetBlackboard (Variables|Default|GetEnemyControllerRef)) (Variables|/Game/ClownsparkleContent/Blueprints/Characters/Enemies/BaseEnemy/BP_BaseEnemyController.BP_BaseEnemyController_C|GetIsDeadTag (Variables|Default|GetEnemyControllerRef)) false))))

(event EventTick
  (params (DeltaSeconds :type Float%20%28single-precision%29))
  (bind _playerref (Variables|Default|GetPlayerRef))
  (bind _widget (Variables|Default|GetWidget))
  (bind _returnvalue (Transformation|GetWorldLocation _widget))
  (bind _followcamera (Variables|/Game/ClownsparkleContent/Blueprints/Characters/Player/BP_Player.BP_Player_C|GetFollowCamera _playerref))
  (bind _returnvalue_2 (Transformation|GetWorldLocation _followcamera))
  (Transformation|SetWorldRotation (Variables|Default|GetWidget) (Math|Rotator|FindLookatRotation (Math|Vector|MakeVector (.x _returnvalue) (.y _returnvalue) 0.0) (Math|Vector|MakeVector (.x _returnvalue_2) (.y _returnvalue_2) 0.0)) false false))

(fn ConstructionScript)

(fn AttackPlayer
  (params (PlayerRef :type BP%20Player%20Object%20Reference))
  (bind _monsterinfo (Variables|Default|GetMonsterInfo))
  (bind _enemydamage (Variables|/Game/ClownsparkleContent/DataStorage/DataAssets/Monsters/PDA_MonsterInformation.PDA_MonsterInformation_C|GetEnemyDamage _monsterinfo))
  (bind _outhit (Collision|LineTraceByChannel (+ (Transformation|GetWorldLocation (Variables|/Script/Engine.Character|GetMesh (Variables|Default|GetPlayerRef))) "0.000000,0.000000,90.000000") (+ (Transformation|GetWorldLocation (Variables|Character|GetMesh)) "0.000000,0.000000,90.000000") "TraceTypeQuery1" false (Utilities|Array|MakeArray self) "Persistent"))
  (bind _asbp_shield (Utilities|Casting|CastToBP_Shield (.hitactor _outhit))
    (:then
      (Default|TakeDamage (Variables|/Game/ClownsparkleContent/Blueprints/Actors/PlayerTools/BP_Shield.BP_Shield_C|GetBP_HealthComponent _asbp_shield) _enemydamage))
    (:CastFailed
      (Default|CallAttacked PlayerRef _enemydamage))))

(fn DropLoot
  (bind _returnvalue (Game|SpawnActorfromClass "/Game/ClownsparkleContent/Blueprints/Actors/Interactables/BP_MonsterLoot.BP_MonsterLoot_C" (Math|Conversions|ToTransform(Vector) (Transformation|GetWorldLocation (Variables|Collision|GetCapsuleComponent))) "Undefined" "MultiplyWithRoot" 0 0))
  (LocalVariables|SetMonsterDropRef _returnvalue)
  (for _array_element (Variables|/Game/ClownsparkleContent/DataStorage/DataAssets/Monsters/PDA_MonsterInformation.PDA_MonsterInformation_C|GetMonsterDrops (Variables|Default|GetMonsterInfo))
    (if (Math|Random|RandomBoolwithWeight (/ (Math|Conversions|ToFloat(Integer) (Utilities|Struct|BreakDropChance _array_element)) 1e+02))
      (Utilities|Array|Add (Variables|/Game/ClownsparkleContent/DataStorage/Components/BP_HarvestableComponent.BP_HarvestableComponent_C|GetDrops (Variables|/Game/ClownsparkleContent/Blueprints/Actors/Interactables/BP_MonsterLoot.BP_MonsterLoot_C|GetBP_HarvestableComponent (LocalVariables|GetMonsterDropRef))) (Utilities|Struct|MakeDropAmount (.ItemToDrop (Utilities|Struct|BreakDropChance _array_element)) (.AmountToSpawn (Utilities|Struct|BreakDropChance _array_element))))))
  (Variables|/Game/ClownsparkleContent/Blueprints/Actors/Interactables/BP_BaseInteractable.BP_BaseInteractable_C|SetInteractTime (LocalVariables|GetMonsterDropRef) (Variables|/Game/ClownsparkleContent/DataStorage/DataAssets/Monsters/PDA_MonsterInformation.PDA_MonsterInformation_C|GetPickupDropDuration (Variables|Default|GetMonsterInfo))))

(fn SetSpeed
  (params (Speed :type Float%20%28double-precision%29))
  (Variables|/Script/Engine.CharacterMovementComponent|SetMaxWalkSpeed (Variables|Character|GetCharacterMovement) Speed))