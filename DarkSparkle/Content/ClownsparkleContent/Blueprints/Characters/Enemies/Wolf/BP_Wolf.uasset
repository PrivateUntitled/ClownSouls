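; Wolf enemy character that performs a pounce attack on the player.
; On BeginPlay it runs the parent setup, caches its AB_Wolf anim instance, disables the hit box collision and binds an event to the pounce attack.
; The pounce's Attack stage switches to charge speed without requested-move acceleration, and Recovery restores acceleration at attack speed.
; Players overlapping the box, when its collision is active, are passed to AttackPlayer.
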(event OnComponentBeginOverlap(Box)
  (params (OverlappedComponent :type Primitive%20Component%20Object%20Reference) (OtherActor :type Actor%20Object%20Reference) (OtherComp :type Primitive%20Component%20Object%20Reference) (OtherBodyIndex :type Integer) (bFromSweep :type Boolean) (SweepResult :type Hit%20Result%20Structure%20%28by%20ref%29))
  (bind _asbp_player (Utilities|Casting|CastToBP_Player OtherActor))
  (CallFunction|AttackPlayer _asbp_player))

(event Custom|DoPounceAttack
  (params (PounceStage :type AttackStages%20Enum :default "NewEnumerator0"))
  (bind _charactermovement (Variables|Character|GetCharacterMovement))
  (switch Utilities|FlowControl|Switch|SwitchonAttackStages PounceStage
    (:NewEnumerator1
      (Variables|/Script/Engine.CharacterMovementComponent|SetbRequestedMoveUseAcceleration _charactermovement false)
      (CallFunction|SetSpeed (Variables|/Game/ClownsparkleContent/DataStorage/DataAssets/Monsters/PDA_MonsterInformation.PDA_MonsterInformation_C|GetChargeMoveSpeed (Variables|Default|GetMonsterInfo))))
    (:NewEnumerator2
      (Variables|/Script/Engine.CharacterMovementComponent|SetbRequestedMoveUseAcceleration _charactermovement true)
      (CallFunction|SetSpeed (Variables|Default|GetAttackSpeed)))))

(event EventBeginPlay
  (|CallParentFunction)
  (Utilities|FlowControl|Sequence
    (:then_0
      (bind _asab_wolf (Utilities|Casting|CastToAB_Wolf (Components|SkeletalMesh|GetAnimInstance (Variables|Character|GetMesh))))
      (Variables|Default|SetWolfAnimInstance _asab_wolf))
    (:then_1
      (Collision|SetCollisionEnabled (Variables|Default|GetBox) "NoCollision"))
    (:then_2
      (EventDispatchers|BindEventtoPounceAttack (EventDispatchers|CreateEvent :!event Custom|DoPounceAttack)))))

(event EventTick
  (params (DeltaSeconds :type Float%20%28single-precision%29)))

(fn ConstructionScript)