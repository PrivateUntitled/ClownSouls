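; Controller for the Wolf enemy that picks which attack the wolf uses.
; ChooseAttack rolls a random index across all WolfAttacks enum entries and writes the result to the WolfAttacks Blackboard key.
; Sizing the roll from the enum's entry count avoids a hard-coded attack total.
; The event graph holds only disabled default nodes, and nothing in this Blueprint calls ChooseAttack.
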(event EventBeginPlay
  (|CallParentFunction) ; This node is disabled and will not be called.\nDrag off pins to build functionality.
)

(event EventTick
  (params (DeltaSeconds :type Float%20%28single-precision%29))
  (|CallParentFunction DeltaSeconds) ; This node is disabled and will not be called.\nDrag off pins to build functionality.
)

(fn ConstructionScript
  (|CallParentFunction))

(fn ChooseAttack
  (AI|Components|Blackboard|SetValueasEnum (Variables|Default|GetBlackboard) (Variables|Default|GetWolfAttacks) (Utilities|Enum|ByteToEnumWolfAttacks (Math|Conversions|ToByte(Integer) (Math|Random|RandomIntegerinRange 0 (- (|GetNumEnumEntries) 1))))))