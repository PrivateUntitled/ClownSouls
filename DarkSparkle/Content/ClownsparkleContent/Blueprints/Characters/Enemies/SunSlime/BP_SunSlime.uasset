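; BP_SunSlime is a slime enemy that latches onto the player and lets go when the player dodges.
; Overlapping its box with the player disables capsule and mesh collision, snaps it to the player's ChestSocket and flags it attached.
; A handler, apparently bound to the player's dodge event, detaches it and restores collision after a brief delay.
; Both transitions set the SunSlime controller's action enum and trigger ChooseAttack.
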(event OnComponentBeginOverlap(Box)
  (params (OverlappedComponent :type Primitive%20Component%20Object%20Reference) (OtherActor :type Actor%20Object%20Reference) (OtherComp :type Primitive%20Component%20Object%20Reference) (OtherBodyIndex :type Integer) (bFromSweep :type Boolean) (SweepResult :type Hit%20Result%20Structure%20%28by%20ref%29))
  (Utilities|Casting|CastToBP_Player OtherActor)
  (Collision|SetCollisionEnabled (Variables|Default|GetCapsuleComponent) "NoCollision")
  (Transformation|AttachActorToActor self (Variables|Default|GetPlayerRef) "ChestSocket" "SnapToTarget" "SnapToTarget" "SnapToTarget" false)
  (Variables|Default|SetNewVar true)
  (bind _asbp_sun_slime_controller (Utilities|Casting|CastToBP_SunSlimeController (Variables|Default|GetEnemyControllerRef)))
  (Variables|/Game/ClownsparkleContent/Blueprints/Characters/Enemies/SunSlime/BP_SunSlimeController.BP_SunSlimeController_C|SetSlimeActions _asbp_sun_slime_controller "NewEnumerator1")
  (Default|ChooseAttack _asbp_sun_slime_controller))

(event Custom|CustomEvent_0
  (params (Action%20States :type DodgeStates%20Enum :default "NewEnumerator0"))
  (if (Variables|Default|GetNewVar)
    (Transformation|DetachFromActor self "KeepWorld" "KeepWorld" "KeepWorld")
    (Utilities|FlowControl|Delay 0.1)
    (Collision|SetCollisionEnabled (Variables|Default|GetCapsuleComponent) "QueryAndPhysics")
    (Variables|Default|SetNewVar false)
    (bind _asbp_sun_slime_controller (Utilities|Casting|CastToBP_SunSlimeController (Variables|Default|GetEnemyControllerRef)))
    (Variables|/Game/ClownsparkleContent/Blueprints/Characters/Enemies/SunSlime/BP_SunSlimeController.BP_SunSlimeController_C|SetSlimeActions _asbp_sun_slime_controller "NewEnumerator0")
    (Default|ChooseAttack _asbp_sun_slime_controller)))

(event EventBeginPlay
  (|CallParentFunction)
  (EventDispatchers|BindEventtoDodge (Variables|Default|GetPlayerRef) (EventDispatchers|CreateEvent :!event Custom|CustomEvent_0)))

(event Collision|EventActorBeginOverlap
  (params (OtherActor :type Actor%20Object%20Reference)))

(event EventTick
  (params (DeltaSeconds :type Float%20%28single-precision%29))
  (|CallParentFunction DeltaSeconds) ; This node is disabled and will not be called.\nDrag off pins to build functionality.
)

(fn ConstructionScript
  (|CallParentFunction))