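; BP_ThornyRose is an enemy character that attacks the player through two hitboxes on its mesh.
; On BeginPlay it attaches both boxes to mesh sockets by index, binds their overlap events and starts them with collision off.
; SetAttackCollission toggles the boxes between query-only and no collision, and CheckCollision calls AttackPlayer when the overlapping actor is a BP_Player.
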(event Custom|CheckCollision
  (params (OverlappedComponent :type Primitive%20Component%20Object%20Reference) (OtherActor :type Actor%20Object%20Reference) (OtherComp :type Primitive%20Component%20Object%20Reference) (OtherBodyIndex :type Integer) (bFromSweep :type Boolean) (SweepResult :type Hit%20Result%20Structure%20%28by%20ref%29))
  (bind _asbp_player (Utilities|Casting|CastToBP_Player OtherActor))
  (CallFunction|AttackPlayer _asbp_player))

(event EventBeginPlay
  (bind _mesh (Variables|Character|GetMesh))
  (bind _mesh_2 (Variables|Character|GetMesh))
  (|CallParentFunction)
  (Transformation|AttachComponentToComponent (Variables|Default|GetBox) _mesh_2 (Variables|/Script/Engine.SkeletalMeshSocket|GetSocketName (Class|SkeletalMesh|GetSocketbyIndex (Variables|/Script/Engine.SkeletalMeshComponent|GetSkeletalMeshAsset _mesh_2))) "SnapToTarget" "KeepRelative" "SnapToTarget" true)
  (Transformation|AttachComponentToComponent (Variables|Default|GetBox1) _mesh (Variables|/Script/Engine.SkeletalMeshSocket|GetSocketName (Class|SkeletalMesh|GetSocketbyIndex (Variables|/Script/Engine.SkeletalMeshComponent|GetSkeletalMeshAsset _mesh) 1)) "SnapToTarget" "KeepRelative" "SnapToTarget" true)
  (Collision|BindEventtoOnComponentBeginOverlap (Variables|Default|GetBox) (EventDispatchers|CreateEvent :!event Custom|CheckCollision))
  (Collision|BindEventtoOnComponentBeginOverlap (Variables|Default|GetBox1) (EventDispatchers|CreateEvent :!event Custom|CheckCollision))
  (Collision|SetCollisionEnabled (Variables|Default|GetBox) "NoCollision"))

(event Collision|EventActorBeginOverlap
  (params (OtherActor :type Actor%20Object%20Reference)))

(event EventTick
  (params (DeltaSeconds :type Float%20%28single-precision%29))
  (|CallParentFunction DeltaSeconds) ; This node is disabled and will not be called.\nDrag off pins to build functionality.
)

(fn ConstructionScript
  (|CallParentFunction))

(fn SetAttackCollission
  (params (SetAttackCollission :type Boolean))
  (if SetAttackCollission
    (Collision|SetCollisionEnabled (Variables|Default|GetBox1) "QueryOnly")
    (else
      (Collision|SetCollisionEnabled (Variables|Default|GetBox1) "NoCollision"))))