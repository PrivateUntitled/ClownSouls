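; AI controller for the Deer enemy that picks which attack it performs by writing it to the Blackboard.
; Shortly after BeginPlay it caches the controlled BP_Deer, and it extends the parent's ChooseAttack.
; A player up to 200 units away along positive world X triggers the kick, regardless of other axes.
; Otherwise a distance threshold selects a random far attack or the close attack.
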(event EventBeginPlay
  (|CallParentFunction)
  (Utilities|FlowControl|Delay 0.1)
  (bind _asbp_deer (Utilities|Casting|CastToBP_Deer (Pawn|GetControlledPawn)))
  (Variables|Default|SetDeerRef _asbp_deer))

(event EventTick
  (params (DeltaSeconds :type Float%20%28single-precision%29))
  (|CallParentFunction DeltaSeconds) ; This node is disabled and will not be called.\nDrag off pins to build functionality.
)

(fn ConstructionScript
  (|CallParentFunction))

(fn ChooseAttack
  (|CallParentFunction)
  (if (Math|Float|InRange(Float) (.X (Math|Vector|BreakVector (- (Transformation|GetWorldLocation (Variables|/Script/Engine.Character|GetMesh (Variables|Default|GetDeerRef))) (Transformation|GetWorldLocation (Variables|/Script/Engine.Character|GetMesh (Variables|Default|GetPlayerRef)))))) -2e+02 0.0)
    (AI|Components|Blackboard|SetValueasEnum (Variables|Default|GetBlackboard) (Variables|Default|GetAttackTag) (Variables|Default|GetKickDeerAttack))
    (elif (<= (Variables|Default|GetDistance) (Math|Vector|Distance(Vector) (Transformation|GetWorldLocation (Variables|/Script/Engine.Character|GetMesh (Variables|Default|GetDeerRef))) (Transformation|GetWorldLocation (Variables|/Script/Engine.Character|GetMesh (Variables|Default|GetPlayerRef)))))
      (AI|Components|Blackboard|SetValueasEnum (Variables|Default|GetBlackboard) (Variables|Default|GetAttackTag) (.OutItem (Utilities|Array|Random (Variables|Default|GetFarAttacks))))
      (else
        (AI|Components|Blackboard|SetValueasEnum (Variables|Default|GetBlackboard) (Variables|Default|GetAttackTag) (Variables|Default|GetCloseAttack))))))