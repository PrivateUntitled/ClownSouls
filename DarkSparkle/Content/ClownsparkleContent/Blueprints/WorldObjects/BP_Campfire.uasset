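; BP_Campfire is a world object that offers itself to the player as the current interactable.
; When its Sphere begins an overlap, it writes itself into the InteractablesInRange reference on BP_Player.
; When the overlap ends, it clears that reference only if it still points to this campfire.
; Both events fetch player pawn 0 without checking which actor overlapped, and the interaction itself is not handled here.
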(event OnComponentBeginOverlap(Sphere)
  (params (OverlappedComponent :type Primitive%20Component%20Object%20Reference) (OtherActor :type Actor%20Object%20Reference) (OtherComp :type Primitive%20Component%20Object%20Reference) (OtherBodyIndex :type Integer) (bFromSweep :type Boolean) (SweepResult :type Hit%20Result%20Structure%20%28by%20ref%29))
  (bind _asbp_player (Utilities|Casting|CastToBP_Player (Game|Player|GetPlayerPawn 0)))
  (Variables|/Game/ClownsparkleContent/Blueprints/Characters/Player/BP_Player.BP_Player_C|SetInteractablesInRange _asbp_player self))

(event OnComponentEndOverlap(Sphere)
  (params (OverlappedComponent :type Primitive%20Component%20Object%20Reference) (OtherActor :type Actor%20Object%20Reference) (OtherComp :type Primitive%20Component%20Object%20Reference) (OtherBodyIndex :type Integer))
  (bind _asbp_player (Utilities|Casting|CastToBP_Player (Game|Player|GetPlayerPawn 0)))
  (if (== (Variables|/Game/ClownsparkleContent/Blueprints/Characters/Player/BP_Player.BP_Player_C|GetInteractablesInRange _asbp_player) self)
    (Variables|/Game/ClownsparkleContent/Blueprints/Characters/Player/BP_Player.BP_Player_C|SetInteractablesInRange _asbp_player 0)))

(event EventBeginPlay)

(event EventTick
  (params (DeltaSeconds :type Float%20%28single-precision%29)))

(fn ConstructionScript)