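; Archived base room game mode that caches the game instance on BeginPlay for use in room and door setup.
; SetRoom and GetRoomType have empty entry points, so their logic is disconnected and never runs.
; That orphaned logic spawns an archived door at each room door transform for every next-room coordinate in the game instance's map generation data, tagging it with its coordinate and looked-up room type.
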(event EventBeginPlay
  (bind _asbp_game_instance (Utilities|Casting|CastToBP_GameInstance (Game|GetGameInstance)))
  (Variables|Default|SetGameInstanceRef _asbp_game_instance))

(event EventTick
  (params (DeltaSeconds :type Float%20%28single-precision%29)))

(fn ConstructionScript)

(fn SetRoom)

(fn GetRoomType
  (params (RoomCoordinate :type Room%20Coordinate%20Structure)))