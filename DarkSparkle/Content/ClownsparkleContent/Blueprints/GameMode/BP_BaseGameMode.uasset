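; Base game mode that runs the biodiversity Dungeoneer timer, loot message queue and initial pickup spawning.
; On BeginPlay it caches the game instance, calculates the biodiversity index and scatters twigs and stones over random, non-reused spawn points.
; A one-second looping timer counts down Dungeoneer time stored in the game instance, resetting it and decrementing the criteria at zero.
; Incoming loot messages are queued, then cleared after a short delay.
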(event Custom|CustomEvent
  (bind _gameinstanceref (Variables|Default|GetGameInstanceRef))
  (bind _biodiversitystats (Variables|/Game/ClownsparkleContent/Blueprints/BP_GameInstance.BP_GameInstance_C|GetBiodiversityStats _gameinstanceref))
  (bind (_dungeoneercriteria _dungeoneertime) (Utilities|Struct|BreakBiodiversityComponents _biodiversitystats))
  (if (> (Utilities|Struct|BreakBiodiversityComponents (Variables|/Game/ClownsparkleContent/Blueprints/BP_GameInstance.BP_GameInstance_C|GetBiodiversityStats (Variables|Default|GetGameInstanceRef))) 0.0)
    (Math|Float|DecrementFloat (Utilities|Struct|BreakBiodiversityComponents (Variables|/Game/ClownsparkleContent/Blueprints/BP_GameInstance.BP_GameInstance_C|GetBiodiversityStats (Variables|Default|GetGameInstanceRef))))
    (else
      (Utilities|Struct|SetmembersinBiodiversityComponents _biodiversitystats _dungeoneertime)
      (Math|Float|DecrementFloat (Math|Float|Max(Float) _dungeoneercriteria 0.0)))))

(event Custom|Message
  (params (NewParam :type Text))
  (Utilities|Array|Add (Variables|Default|GetLootMessages) NewParam)
  (CallFunction|Countdown))

(event Custom|Countdown
  (Utilities|FlowControl|Delay 3.0)
  (bind _arrayelement (Utilities|Array|ReverseforEachLoop (Variables|Default|GetLootMessages) :!label _label)
    (:LoopBody
      (Utilities|Array|RemoveItem (Variables|Default|GetLootMessages) _arrayelement))
    (:Completed
      (Utilities|FlowControl|Delay 0.2)
      (if (!= (Utilities|Array|Length (Variables|Default|GetLootMessages)) 0)
        (goto _label)))))

(event EventBeginPlay
  (bind _asbp_game_instance (Utilities|Casting|CastToBP_GameInstance (Game|GetGameInstance)))
  (Variables|Default|SetGameInstanceRef _asbp_game_instance)
  (Utilities|Time|SetTimerbyEvent (delegate Custom|CustomEvent) 1.0 true)
  (Default|CalculateBiodiversityIndex (Variables|Default|GetGameInstanceRef))
  (EventDispatchers|BindEventtoAddLootMessage (delegate Custom|Message))
  (CallFunction|SpawnPickup "/Game/ClownsparkleContent/Blueprints/Actors/Interactables/BP_Twig.BP_Twig_C" 2)
  (CallFunction|SpawnPickup "/Game/ClownsparkleContent/Blueprints/Actors/Interactables/BP_Stone.BP_Stone_C" 2))

(event EventTick
  (params (DeltaSeconds :type Float%20%28single-precision%29)))

(fn ConstructionScript)

(fn SpawnPickup
  (params (ItemToSpawn :type BP%20Base%20Interactable%20Class%20Reference) (AmountToSpawn :type Integer))
  (for _index (range 0 (Math|Integer|Min(Integer) AmountToSpawn (- (Utilities|Array|Length (Variables|Default|GetSpawnpointPickup)) 1)))
    (LocalVariables|SetNewLocalVar (.OutItem (Utilities|Array|Random (Variables|Default|GetSpawnpointPickup))))
    (Game|SpawnActorfromClass ItemToSpawn (Math|Conversions|ToTransform(Vector) (Transformation|GetWorldLocation (Variables|/Script/Engine.Actor|GetRootComponent (LocalVariables|GetNewLocalVar)))) "Undefined" "MultiplyWithRoot" 0 0)
    (Utilities|Array|RemoveItem (Variables|Default|GetSpawnpointPickup) (LocalVariables|GetNewLocalVar))))