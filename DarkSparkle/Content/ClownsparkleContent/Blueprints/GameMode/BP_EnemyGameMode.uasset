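; Enemy game mode that populates a room with monsters and tracks their counts for the biodiversity system.
; BeginPlay refreshes the game instance's biodiversity index, then picks the current room's enemy type, or a random one without room data.
; SpawnMonsters records a randomized count and spawns through random spawn-point components.
; CalculateIndex, uncalled here, maps survival ratios to per-species biodiversity percentages, though its low-ratio branch passes BaseEnemy, which matches no species.
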(event EventBeginPlay
  (|CallParentFunction)
  (bind _asbp_game_instance (Utilities|Casting|CastToBP_GameInstance (Game|GetGameInstance)))
  (Variables|Default|SetGameInstanceRef _asbp_game_instance)
  (Default|CalculateBiodiversityIndex (Variables|Default|GetGameInstanceRef))
  (if (== (Utilities|Array|Length (.RoomGeneration (Utilities|Struct|BreakMapGeneration (Variables|/Game/ClownsparkleContent/Blueprints/BP_GameInstance.BP_GameInstance_C|GetMapStruct (Variables|Default|GetGameInstanceRef))))) 0)
    (CallFunction|SpawnMonsters (.OutItem (Utilities|Array|Random (Variables|Default|GetSpawnableMonsters))))
    (else
      (switch Utilities|FlowControl|Switch|SwitchonEnemyType (Utilities|Struct|BreakRoomGeneration (Utilities|Array|Get(acopy) (.RoomGeneration (Utilities|Struct|BreakMapGeneration (Variables|/Game/ClownsparkleContent/Blueprints/BP_GameInstance.BP_GameInstance_C|GetMapStruct (Variables|Default|GetGameInstanceRef)))) (.CurrentRoom (Utilities|Struct|BreakMapGeneration (Variables|/Game/ClownsparkleContent/Blueprints/BP_GameInstance.BP_GameInstance_C|GetMapStruct (Variables|Default|GetGameInstanceRef))))))
        (:NewEnumerator2
          (CallFunction|SpawnMonsters "/Game/ClownsparkleContent/DataStorage/DataAssets/Monsters/DA_Wolf.DA_Wolf"))
        (:NewEnumerator3
          (CallFunction|SpawnMonsters "/Game/ClownsparkleContent/DataStorage/DataAssets/Monsters/DA_Deer.DA_Deer"))
        (:NewEnumerator5
          (CallFunction|SpawnMonsters "/Game/ClownsparkleContent/DataStorage/DataAssets/Monsters/DA_SunSlime.DA_SunSlime"))))))

(event EventTick
  (params (DeltaSeconds :type Float%20%28single-precision%29))
  (|CallParentFunction DeltaSeconds) ; This node is disabled and will not be called.\nDrag off pins to build functionality.
)

(fn ConstructionScript
  (|CallParentFunction))

(fn SpawnMonsters
  (params (ChosenMonster :type PDA%20Monster%20Information%20Object%20Reference))
  (bind _spawnpoints (Variables|Default|GetSpawnpoints))
  (bind _outitem (Utilities|Array|Random _spawnpoints))
  (bind _output_get (LocalVariables|SetSpawnAmount (Math|Random|RandomIntegerinRange (Variables|/Game/ClownsparkleContent/DataStorage/DataAssets/Monsters/PDA_MonsterInformation.PDA_MonsterInformation_C|GetMinSpawnAmount ChosenMonster) (Variables|/Game/ClownsparkleContent/DataStorage/DataAssets/Monsters/PDA_MonsterInformation.PDA_MonsterInformation_C|GetMaxSpawnAmount ChosenMonster))))
  (Utilities|Array|Add (Variables|Default|GetEnemyCounter) (Utilities|Struct|MakeEnemyCounter (Variables|/Game/ClownsparkleContent/DataStorage/DataAssets/Monsters/PDA_MonsterInformation.PDA_MonsterInformation_C|GetEnemyType ChosenMonster) _output_get _output_get))
  (for _index (range 1 (LocalVariables|GetSpawnAmount))
    (Utilities|IsValid _outitem
      (:Is%20Valid
        (Default|SpawnEnemy (Actor|GetComponentbyClass _outitem "/Game/ClownsparkleContent/DataStorage/Components/BP_EnemySpawnPoint.BP_EnemySpawnPoint_C") (Variables|/Game/ClownsparkleContent/DataStorage/DataAssets/Monsters/PDA_MonsterInformation.PDA_MonsterInformation_C|GetEnemyClass ChosenMonster))))))

(fn CalculateIndex
  (for _array_element (Variables|Default|GetEnemyCounter)
    (if (Math|Float|InRange(Float) (/ (Math|Conversions|ToFloat(Integer) (.CurrentAmount (Utilities|Struct|BreakEnemyCounter _array_element))) (Math|Conversions|ToFloat(Integer) (.MaxAmount (Utilities|Struct|BreakEnemyCounter _array_element)))) 0.66 1.0 false)
      (CallFunction|NewFunction0 (.EnemyType (Utilities|Struct|BreakEnemyCounter _array_element)) 0.04)
      (elif (not (Math|Float|InRange(Float) (/ (Math|Conversions|ToFloat(Integer) (.CurrentAmount (Utilities|Struct|BreakEnemyCounter _array_element))) (Math|Conversions|ToFloat(Integer) (.MaxAmount (Utilities|Struct|BreakEnemyCounter _array_element)))) 0.33 0.66 false))
        (CallFunction|NewFunction0 "NewEnumerator0" -0.04)))))

(fn NewFunction0
  (params (EnemyTypes :type EnemyType%20Enum :default "NewEnumerator0") (IncreasePercent :type Float%20%28double-precision%29))
  (bind _returnvalue (+ IncreasePercent 1.0))
  (bind _gameinstanceref (Variables|Default|GetGameInstanceRef))
  (bind _returnvalue_2 (Math|Float|Clamp(Float) _returnvalue 0.0 0.08))
  (bind _biodiversitystats (Variables|/Game/ClownsparkleContent/Blueprints/BP_GameInstance.BP_GameInstance_C|GetBiodiversityStats _gameinstanceref))
  (bind (_wolfcriteria _deercriteria _sunslimecriteria _rosecriteria) (Utilities|Struct|BreakBiodiversityComponents _biodiversitystats))
  (switch Utilities|FlowControl|Switch|SwitchonEnemyType EnemyTypes
    (:NewEnumerator2
      (Utilities|Struct|SetmembersinEnemyComponent _wolfcriteria _returnvalue_2))
    (:NewEnumerator3
      (Utilities|Struct|SetmembersinEnemyComponent _deercriteria _returnvalue_2))
    (:NewEnumerator5
      (Utilities|Struct|SetmembersinEnemyComponent _sunslimecriteria _returnvalue_2))
    (:NewEnumerator6
      (Utilities|Struct|SetmembersinEnemyComponent _rosecriteria _returnvalue_2))))