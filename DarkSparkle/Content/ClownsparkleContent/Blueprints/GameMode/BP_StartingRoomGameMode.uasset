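; Game mode for the starting room that brings up the map and sets the player's mode when play begins.
; BeginPlay caches the BP_GameInstance, creates a BP_Map widget, adds it to the viewport and tells it to generate the map.
; It then switches BP_PlayerController to a fixed player mode, with no per-frame logic.
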(event EventBeginPlay
  (bind _asbp_game_instance (Utilities|Casting|CastToBP_GameInstance (Game|GetGameInstance)))
  (Variables|Default|SetGameInstanceRef _asbp_game_instance)
  (bind _returnvalue (UserInterface|CreateWidget "/Game/ClownsparkleContent/Blueprints/Widgets/BP_Map.BP_Map_C"))
  (UserInterface|Viewport|AddtoViewport _returnvalue 1)
  (Default|GenerateMap _returnvalue)
  (bind _asbp_player_controller (Utilities|Casting|CastToBP_PlayerController (Game|GetPlayerController 0)))
  (Default|SetPlayerMode _asbp_player_controller "NewEnumerator2"))

(event EventTick
  (params (DeltaSeconds :type Float%20%28single-precision%29))
  (|CallParentFunction DeltaSeconds) ; This node is disabled and will not be called.\nDrag off pins to build functionality.
)

(fn ConstructionScript
  (|CallParentFunction))