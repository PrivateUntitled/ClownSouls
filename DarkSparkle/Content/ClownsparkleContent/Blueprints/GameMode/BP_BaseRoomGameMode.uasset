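; Base game mode for room levels that handles the map display, exit doors and a kill counter.
; On BeginPlay it caches the game instance, shows an animated map widget and sets the player controller's mode.
; SetRoom spawns a door at each RoomDoors transform for the next room coordinates, tagged with the type GetRoomType finds in the generated map data.
; UpdateDifficulty counts kills and sets a game instance flag past a threshold.
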(event EventBeginPlay
  (bind _asbp_game_instance (Utilities|Casting|CastToBP_GameInstance (Game|GetGameInstance)))
  (Variables|Default|SetGameInstanceRef _asbp_game_instance)
  (bind _returnvalue (UserInterface|CreateWidget "/Game/ClownsparkleContent/Blueprints/Widgets/BP_Map.BP_Map_C"))
  (Default|ShowMapAnimation _returnvalue)
  (UserInterface|Viewport|AddtoViewport _returnvalue 1)
  (bind _asbp_player_controller (Utilities|Casting|CastToBP_PlayerController (Game|GetPlayerController 0)))
  (Default|SetPlayerMode _asbp_player_controller "NewEnumerator2"))

(event EventTick
  (params (DeltaSeconds :type Float%20%28single-precision%29)))

(fn ConstructionScript)

(fn SetRoom
  (for (_array_element _array_index) (Utilities|Struct|BreakMapGenerationStruct (Variables|/Game/ClownsparkleContent/Blueprints/BP_GameInstance.BP_GameInstance_C|GetMapGeneration (Variables|Default|GetGameInstanceRef)))
    (bind _coordinateroomtype (CallFunction|GetRoomType _array_element))
    (bind _returnvalue (Game|SpawnActorfromClass "/Game/ClownsparkleContent/Blueprints/Actors/BP_Door.BP_Door_C" (Transformation|GetWorldTransform (Variables|/Script/Engine.Actor|GetRootComponent (Utilities|Array|Get(acopy) (Variables|Default|GetRoomDoors) _array_index))) "Undefined" "MultiplyWithRoot" 0 0))
    (Variables|/Game/ClownsparkleContent/Blueprints/Actors/BP_Door.BP_Door_C|SetRoomType _returnvalue _coordinateroomtype)
    (Variables|/Game/ClownsparkleContent/Blueprints/Actors/BP_Door.BP_Door_C|SetRoomCoordinate _returnvalue _array_element)))

(fn GetRoomType
  (params (RoomCoordinate :type Room%20Coordinate%20Structure))
  (for _array_element (Utilities|Struct|BreakMapGenerationStruct (Variables|/Game/ClownsparkleContent/Blueprints/BP_GameInstance.BP_GameInstance_C|GetMapGeneration (Variables|Default|GetGameInstanceRef)))
    (if (and (Utilities|Enum|Equal(Enum) (.roomx RoomCoordinate) (.roomx (.RoomNumber (Utilities|Struct|BreakRoomTypeStorage _array_element)))) (Utilities|Enum|Equal(Enum) (.roomy (.RoomNumber (Utilities|Struct|BreakRoomTypeStorage _array_element))) (.roomy RoomCoordinate)))
      (return (.RoomType (Utilities|Struct|BreakRoomTypeStorage _array_element))))))

(fn UpdateDifficulty
  (bind _killsamount (Variables|Default|GetKillsAmount))
  (Math|Integer|IncrementInt _killsamount
    (:%20%20
      (if (> _killsamount 3)
        (Variables|/Game/ClownsparkleContent/Blueprints/BP_GameInstance.BP_GameInstance_C|SetNewVar (Variables|Default|GetGameInstanceRef) true)))))