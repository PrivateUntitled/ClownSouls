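; BP_Sword is the player's melee weapon, damaging overlapped enemies that are not invincible.
; It caches the player and controller, starts with mesh collision off and binds to the player's Attacking dispatcher, with handler events toggling query-only collision as a hit window.
; Overlaps pass the player's BaseDamage to the enemy's attacked call.
; An outdated heavy-attack path with strength-scaled damage and animation-timed collision remains, its binding never run.
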(event OnComponentBeginOverlap(StaticMesh)
  (params (OverlappedComponent :type Primitive%20Component%20Object%20Reference) (OtherActor :type Actor%20Object%20Reference) (OtherComp :type Primitive%20Component%20Object%20Reference) (OtherBodyIndex :type Integer) (bFromSweep :type Boolean) (SweepResult :type Hit%20Result%20Structure%20%28by%20ref%29))
  (bind _asbp_base_enemy (Utilities|Casting|CastToBP_BaseEnemy OtherActor))
  (if (not (Variables|/Game/ClownsparkleContent/Blueprints/Characters/Enemies/BaseEnemy/BP_BaseEnemy.BP_BaseEnemy_C|GetInvincible _asbp_base_enemy))
    (Default|CallAttacked _asbp_base_enemy (Variables|/Game/ClownsparkleContent/Blueprints/Characters/Player/BP_Player.BP_Player_C|GetBaseDamage (Variables|Default|GetPlayerRef)))))

(event Custom|DoHeavyAttack
  (bind _playerref (Variables|Default|GetPlayerRef))
  ;[1 0.06771 0.06771] [Archived/Outdated] Heavy Attack
  (CallFunction|CalculateTotalDamage (Variables|/Game/ClownsparkleContent/Blueprints/Characters/Player/BP_Player.BP_Player_C|GetHeavyDamageMultiplier _playerref))
  (bind _asnew_anim_blueprint (Utilities|Casting|CastToNewAnimBlueprint (Components|SkeletalMesh|GetAnimInstance (Variables|/Script/Engine.Character|GetMesh _playerref))))
  (Collision|SetCollisionEnabled (Variables|Default|GetStaticMesh) "QueryOnly")
  (bind _heavyattackduration (Default|GetHeavyAttackDuration _asnew_anim_blueprint))
  (Utilities|FlowControl|Delay _heavyattackduration)
  (Collision|SetCollisionEnabled (Variables|Default|GetStaticMesh) "NoCollision"))

(event Custom|EnableCollission
  (params (NewParam :type AttackStages%20Enum :default "NewEnumerator0"))
  (if (Utilities|Enum|Equal(Enum) NewParam "NewEnumerator1")
    (Collision|SetCollisionEnabled (Variables|Default|GetStaticMesh) "QueryOnly")
    (else
      (Collision|SetCollisionEnabled (Variables|Default|GetStaticMesh) "NoCollision"))))

(event Custom|SetCollission
  (params (EnableAttack :type Boolean))
  (if EnableAttack
    (Collision|SetCollisionEnabled (Variables|Default|GetStaticMesh) "QueryOnly")
    (else
      (Collision|SetCollisionEnabled (Variables|Default|GetStaticMesh) "NoCollision"))))

(event EventBeginPlay
  (Utilities|FlowControl|Sequence
    (:then_0
      (bind _asbp_player (Utilities|Casting|CastToBP_Player (Game|Player|GetPlayerPawn 0)))
      (Variables|Default|SetPlayerRef _asbp_player)
      (bind _asbp_player_controller (Utilities|Casting|CastToBP_PlayerController (Game|GetPlayerController 0)))
      (Variables|Default|SetPlayerControllerRef _asbp_player_controller))
    (:then_1
      (Collision|SetCollisionEnabled (Variables|Default|GetStaticMesh) "NoCollision"))
    (:then_2
      (EventDispatchers|BindEventtoAttacking (Variables|Default|GetPlayerRef) (EventDispatchers|CreateEvent :!event Custom|SetCollission)))))

(event EventTick
  (params (DeltaSeconds :type Float%20%28single-precision%29)))

(fn ConstructionScript)

(fn CalculateTotalDamage
  (params (DamageMultiplier :type Float%20%28double-precision%29))
  (bind _playerref (Variables|Default|GetPlayerRef))
  (Variables|Default|SetTotalDamage (* DamageMultiplier (Math|Conversions|ToFloat(Integer) (+ (Variables|/Game/ClownsparkleContent/Blueprints/Characters/Player/BP_Player.BP_Player_C|GetBaseDamage _playerref) (Variables|/Game/ClownsparkleContent/Blueprints/Characters/Player/BP_Player.BP_Player_C|GetStrength _playerref))))))