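; BP_Shield is the player's shield tool, used for blocking and for damaging enemies on contact.
; Player block and attack events drive it, toggling box collision and contact damage, with a controller-run cooldown for the shield.
; While lowered with blocking enabled, a delayed loop regenerates its health component by a base amount plus a tenth of the player's current health.
; Cube1 overlaps deal the player's base damage to non-invincible enemies when damage is enabled.
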(event OnComponentBeginOverlap(Cube1)
  (params (OverlappedComponent :type Primitive%20Component%20Object%20Reference) (OtherActor :type Actor%20Object%20Reference) (OtherComp :type Primitive%20Component%20Object%20Reference) (OtherBodyIndex :type Integer) (bFromSweep :type Boolean) (SweepResult :type Hit%20Result%20Structure%20%28by%20ref%29))
  (bind _asbp_base_enemy (Utilities|Casting|CastToBP_BaseEnemy OtherActor))
  (if (and (not (Variables|/Game/ClownsparkleContent/Blueprints/Characters/Enemies/BaseEnemy/BP_BaseEnemy.BP_BaseEnemy_C|GetInvincible _asbp_base_enemy)) (Variables|Default|GetDealDamage))
    (Default|CallAttacked _asbp_base_enemy (Variables|/Game/ClownsparkleContent/Blueprints/Characters/Player/BP_Player.BP_Player_C|GetBaseDamage (Variables|References|GetPlayerRef)))))

(event Custom|ShieldCooldown
  (Default|ShieldCooldown (Variables|References|GetPlayerControllerRef) (Variables|Default|GetDuration)))

(event Custom|CustomEvent
  (params (EnableAttack :type Boolean))
  (Variables|Default|SetDealDamage EnableAttack))

(event Custom|UpdateShield
  (params (NewParam :type ActionStates%20Enum :default "NewEnumerator0"))
  (bind _box (Variables|Default|GetBox))
  (bind _bp_healthcomponent (Variables|Default|GetBP_HealthComponent))
  (Utilities|FlowControl|Sequence
    (:then_0
      ;[0.08854 0.08854 0.08854] Set Shield Collision
      (if (Utilities|Enum|Equal(Enum) NewParam "NewEnumerator0")
        (Collision|SetCollisionEnabled _box "QueryOnly")
        (else
          (Collision|SetCollisionEnabled _box "NoCollision"))))
    (:then_1
      ;[0.05208 0.05208 0.05208] Reciver Shield Energy When Shield is Down
      (if (Math|Boolean|ANDBoolean (< (Variables|/Game/ClownsparkleContent/DataStorage/Components/BP_HealthComponent.BP_HealthComponent_C|GetHealth _bp_healthcomponent) (Variables|/Game/ClownsparkleContent/DataStorage/Components/BP_HealthComponent.BP_HealthComponent_C|GetMaxHealth _bp_healthcomponent)) (Utilities|Enum|Equal(Enum) NewParam "NewEnumerator1") (Utilities|Struct|BreakPlayerFunctionality (Variables|/Game/ClownsparkleContent/Blueprints/Controllers/BP_PlayerController.BP_PlayerController_C|GetPlayerFunctionality (Variables|References|GetPlayerControllerRef)))) :!label _label
        (Utilities|FlowControl|Delay 1.0)
        (Default|Heal (Variables|Default|GetBP_HealthComponent) (+ (Variables|Default|GetBaseHeal) (Math|Float|Truncate (* (Variables|/Game/ClownsparkleContent/DataStorage/Components/BP_HealthComponent.BP_HealthComponent_C|GetHealth (Variables|/Game/ClownsparkleContent/Blueprints/Characters/Player/BP_Player.BP_Player_C|GetHealthComponent (Variables|References|GetPlayerRef))) 0.1))))
        (goto _label)))))

(event EventBeginPlay
  (EventDispatchers|BindEventtoOnDeath (Variables|Default|GetBP_HealthComponent) (EventDispatchers|CreateEvent :!event Custom|ShieldCooldown))
  (bind _asbp_player_controller (Utilities|Casting|CastToBP_PlayerController (Game|GetPlayerController 0)))
  (Variables|References|SetPlayerControllerRef _asbp_player_controller)
  (bind _asbp_player (Utilities|Casting|CastToBP_Player (Game|Player|GetPlayerPawn 0)))
  (Variables|References|SetPlayerRef _asbp_player)
  (EventDispatchers|BindEventtoBlock (Variables|References|GetPlayerRef) (EventDispatchers|CreateEvent :!event Custom|UpdateShield))
  (EventDispatchers|BindEventtoAttacking (Variables|References|GetPlayerRef) (EventDispatchers|CreateEvent :!event Custom|CustomEvent)))

(event Collision|EventActorBeginOverlap
  (params (OtherActor :type Actor%20Object%20Reference)))

(event EventTick
  (params (DeltaSeconds :type Float%20%28single-precision%29)))

(fn ConstructionScript)