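; Base interactable actor that registers itself with the player as the interactable currently in range.
; On BeginPlay it caches the BP_Player pawn and binds OnInteract, left empty here, to the Interact event.
; Sphere begin overlap writes itself into the player's single InteractablesInRange reference without checking the overlapping actor.
; End overlap clears that reference only if it still points to this actor.
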(event OnComponentEndOverlap(Sphere)
  (params (OverlappedComponent :type Primitive%20Component%20Object%20Reference) (OtherActor :type Actor%20Object%20Reference) (OtherComp :type Primitive%20Component%20Object%20Reference) (OtherBodyIndex :type Integer))
  (if (== (Variables|/Game/ClownsparkleContent/Blueprints/Characters/Player/BP_Player.BP_Player_C|GetInteractablesInRange (Variables|Default|GetPlayerRef)) self)
    (Variables|/Game/ClownsparkleContent/Blueprints/Characters/Player/BP_Player.BP_Player_C|SetInteractablesInRange (Variables|Default|GetPlayerRef) 0)))

(event OnComponentBeginOverlap(Sphere)
  (params (OverlappedComponent :type Primitive%20Component%20Object%20Reference) (OtherActor :type Actor%20Object%20Reference) (OtherComp :type Primitive%20Component%20Object%20Reference) (OtherBodyIndex :type Integer) (bFromSweep :type Boolean) (SweepResult :type Hit%20Result%20Structure%20%28by%20ref%29))
  (Variables|/Game/ClownsparkleContent/Blueprints/Characters/Player/BP_Player.BP_Player_C|SetInteractablesInRange (Variables|Default|GetPlayerRef) self))

(event Custom|OnInteract)

(event EventBeginPlay
  (bind _asbp_player (Utilities|Casting|CastToBP_Player (Game|Player|GetPlayerPawn 0)))
  (Variables|Default|SetPlayerRef _asbp_player)
  (EventDispatchers|BindEventtoInteract (delegate Custom|OnInteract)))

(event Collision|EventActorBeginOverlap
  (params (OtherActor :type Actor%20Object%20Reference)))

(event EventTick
  (params (DeltaSeconds :type Float%20%28single-precision%29)))

(fn ConstructionScript)