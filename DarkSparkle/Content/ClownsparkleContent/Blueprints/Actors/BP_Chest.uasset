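; Interactable chest that opens once when the player interacts with it and announces a random reward.
; Interaction, inherited from a parent class, plays a timeline that swings a mesh open by lerping its world rotation, then sets an opened flag.
; A random roll up to a reward-count variable picks a health potion or food ration message, which is only printed, with no items granted.
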(event EventBeginPlay
  (|CallParentFunction))

(event EventOnInteract
  (|CallParentFunction)
  (if (not (Variables|Default|GetIsChestOpened))
    (Utilities|FlowControl|Sequence
      (:then_0
        (bind _alpha (Timeline|Timeline Play)
          (:Update
            (Transformation|SetWorldRotation (Variables|Default|GetStaticMesh2) (Math|Rotator|Lerp(Rotator) "0, 0, 0" "0.000000,0.000000,-130.000000" _alpha) false false))))
      (:then_1
        (Variables|Default|SetIsChestOpened true))
      (:then_2
        (switch int (Math|Random|RandomIntegerinRange 0 (Variables|Default|GetDifferentRewards))
          (:0
            (Development|PrintString "You gained Health Potions"))
          (:1
            (Development|PrintString "You gained Food Rations"))
          (:2
            (Development|PrintString "You gained Food Rations")))))))

(fn ConstructionScript)