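; BP_ClimableWall is a wall actor that the player starts climbing on contact.
; When its StaticMesh is hit by a BP_Player that is not already climbing, it compares the player capsule's distance to two arrow components.
; It stores the farther arrow's rotation as WallRotation to suit the side of approach, then calls the player's CallClimb with itself as the wall reference.
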(event OnComponentHit(StaticMesh)
  (params (HitComponent :type Primitive%20Component%20Object%20Reference) (OtherActor :type Actor%20Object%20Reference) (OtherComp :type Primitive%20Component%20Object%20Reference) (NormalImpulse :type Vector :default "0, 0, 0") (Hit :type Hit%20Result%20Structure%20%28by%20ref%29))
  (bind _asbp_player (Utilities|Casting|CastToBP_Player OtherActor))
  (if (not (Utilities|Struct|BreakPlayerFunctionality (Variables|/Game/ClownsparkleContent/Blueprints/Controllers/BP_PlayerController.BP_PlayerController_C|GetPlayerFunctionality (Variables|/Game/ClownsparkleContent/Blueprints/Characters/Player/BP_Player.BP_Player_C|GetPlayerControllerRef _asbp_player))))
    (Utilities|FlowControl|Sequence
      (:then_0
        (Math|Float|CompareFloat (Math|Vector|Distance(Vector) (Transformation|GetWorldLocation (Variables|Default|GetArrow1)) (Transformation|GetWorldLocation (Variables|/Script/Engine.Character|GetCapsuleComponent _asbp_player))) (Math|Vector|Distance(Vector) (Transformation|GetWorldLocation (Variables|Default|GetArrow)) (Transformation|GetWorldLocation (Variables|/Script/Engine.Character|GetCapsuleComponent _asbp_player)))
          (:>
            (Variables|Default|SetWallRotation (Transformation|GetWorldRotation (Variables|Default|GetArrow1))))
          (:<
            (Variables|Default|SetWallRotation (Transformation|GetWorldRotation (Variables|Default|GetArrow))))))
      (:then_1
        (Default|CallClimb _asbp_player "NewEnumerator0" self)))))

(event EventBeginPlay)

(event Collision|EventActorBeginOverlap
  (params (OtherActor :type Actor%20Object%20Reference)))

(event EventTick
  (params (DeltaSeconds :type Float%20%28single-precision%29)))

(fn ConstructionScript)