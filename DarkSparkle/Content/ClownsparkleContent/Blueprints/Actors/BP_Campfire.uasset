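; BP_Campfire is an interactable campfire that restocks the player's health potions and heals them.
; BeginPlay and OnInteract call their parent implementations, then interaction runs both effects in sequence.
; Potions increase by a set amount, capped at the carried maximum.
; The health component's Heal receives current health plus a percentage of max health, capped at max health, rather than just the increment.
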(event EventBeginPlay
  (|CallParentFunction))

(event EventOnInteract
  (bind _playerref (Variables|Default|GetPlayerRef))
  (bind _playerref_2 (Variables|Default|GetPlayerRef))
  (bind _bp_healthcomponent (Variables|/Game/ClownsparkleContent/Blueprints/Characters/Player/BP_Player.BP_Player_C|GetBP_HealthComponent _playerref))
  (bind _healthpotion (Variables|/Game/ClownsparkleContent/Blueprints/Characters/Player/BP_Player.BP_Player_C|GetHealthPotion _playerref_2))
  (bind (_amount _maxamount) (Utilities|Struct|BreakHealthPotionStruct _healthpotion))
  (|CallParentFunction)
  (Utilities|FlowControl|Sequence
    (:then_0
      ;[0.3229 0.3229 0.3229] Add Health Potions
      (Utilities|Struct|SetmembersinHealthPotionStruct (Variables|/Game/ClownsparkleContent/Blueprints/Characters/Player/BP_Player.BP_Player_C|GetHealthPotion (Variables|Default|GetPlayerRef)) (Math|Integer|Min(Integer) (+ (Variables|Default|GetHealthPotionsToAdd) _amount) _maxamount)))
    (:then_1
      ;[0.3385 0.3163 0.3095] Heal Player
      (Default|Heal (Variables|/Game/ClownsparkleContent/Blueprints/Characters/Player/BP_Player.BP_Player_C|GetBP_HealthComponent (Variables|Default|GetPlayerRef)) (Math|Integer|Min(Integer) (+ (Variables|/Game/ClownsparkleContent/DataStorage/Components/BP_HealthComponent.BP_HealthComponent_C|GetHealth _bp_healthcomponent) (Math|Float|Truncate (* (Variables|Default|GetHealPercent) (Math|Conversions|ToFloat(Integer) (/ (Variables|/Game/ClownsparkleContent/DataStorage/Components/BP_HealthComponent.BP_HealthComponent_C|GetMaxHealth _bp_healthcomponent) 100))))) (Variables|/Game/ClownsparkleContent/DataStorage/Components/BP_HealthComponent.BP_HealthComponent_C|GetMaxHealth (Variables|/Game/ClownsparkleContent/Blueprints/Characters/Player/BP_Player.BP_Player_C|GetBP_HealthComponent (Variables|Default|GetPlayerRef))))))))

(fn ConstructionScript)