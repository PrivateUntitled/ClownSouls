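; BP_Door is a room-exit door that sends the player to the next room of a generated map.
; On BeginPlay it reads the next room type from the map struct in BP_GameInstance, generating the map after a short delay if none exists.
; When BP_Player overlaps its box, it advances the current room and opens the level matching that type.
; Travel rooms come from a level array, using a travel-room counter clamped to the last entry.
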(event OnComponentBeginOverlap(Box)
  (params (OverlappedComponent :type Primitive%20Component%20Object%20Reference) (OtherActor :type Actor%20Object%20Reference) (OtherComp :type Primitive%20Component%20Object%20Reference) (OtherBodyIndex :type Integer) (bFromSweep :type Boolean) (SweepResult :type Hit%20Result%20Structure%20%28by%20ref%29))
  (bind _gameinstanceref (Variables|Default|GetGameInstanceRef))
  (bind _level (Variables|Default|GetLevel))
  (bind _mapstruct (Variables|/Game/ClownsparkleContent/Blueprints/BP_GameInstance.BP_GameInstance_C|GetMapStruct _gameinstanceref))
  (bind (_mapgeneration _currentroom _travelroomindex) (Utilities|Struct|BreakMapGeneration _mapstruct))
  (Utilities|Casting|CastToBP_Player OtherActor)
  (Utilities|FlowControl|Sequence
    (:then_0
      (Math|Integer|IncrementInt _currentroom
        (:%20%20
          (if (Utilities|Enum|Equal(Enum) (Utilities|Array|Get(acopy) _mapgeneration _currentroom) "NewEnumerator13")
            (Math|Integer|IncrementInt _travelroomindex)))))
    (:then_1
      (switch Utilities|FlowControl|Switch|SwitchonRoomType (Variables|Default|GetNextRoomType)
        (:NewEnumerator6
          (Game|OpenLevel(byName) "FlameOfRespite"))
        (:NewEnumerator0
          (Game|OpenLevel(byName) "MonsterRoom"))
        (:NewEnumerator1
          (Game|OpenLevel(byName) "BossRoom"))
        (:NewEnumerator4
          (Game|OpenLevel(byName) "MonsterDen"))
        (:NewEnumerator5
          (Game|OpenLevel(byName) "ChestRoom"))
        (:NewEnumerator13
          (Game|OpenLevel(byObjectReference) (Utilities|Array|Get(acopy) _level (Math|Integer|Min(Integer) (- (Utilities|Array|Length _level) 1) (Utilities|Struct|BreakMapGeneration (Variables|/Game/ClownsparkleContent/Blueprints/BP_GameInstance.BP_GameInstance_C|GetMapStruct (Variables|Default|GetGameInstanceRef)))))))
        (:NewEnumerator14
          (Game|OpenLevel(byName) "StartingRoom"))))))

(event EventBeginPlay
  (bind _asbp_game_instance (Utilities|Casting|CastToBP_GameInstance (Game|GetGameInstance)))
  (Variables|Default|SetGameInstanceRef _asbp_game_instance)
  (if (.IsGenerated (Utilities|Struct|BreakMapGeneration (Variables|/Game/ClownsparkleContent/Blueprints/BP_GameInstance.BP_GameInstance_C|GetMapStruct (Variables|Default|GetGameInstanceRef))))
    (Variables|Default|SetNextRoomType (Utilities|Array|Get(acopy) (.MapGeneration (Utilities|Struct|BreakMapGeneration (Variables|/Game/ClownsparkleContent/Blueprints/BP_GameInstance.BP_GameInstance_C|GetMapStruct (Variables|Default|GetGameInstanceRef)))) (+ (.CurrentRoom (Utilities|Struct|BreakMapGeneration (Variables|/Game/ClownsparkleContent/Blueprints/BP_GameInstance.BP_GameInstance_C|GetMapStruct (Variables|Default|GetGameInstanceRef)))) 1)))
    (else
      (Utilities|FlowControl|Delay 0.1)
      (Default|GenerateMap (Variables|Default|GetGameInstanceRef))
      (Variables|Default|SetNextRoomType (Utilities|Array|Get(acopy) (.MapGeneration (Utilities|Struct|BreakMapGeneration (Variables|/Game/ClownsparkleContent/Blueprints/BP_GameInstance.BP_GameInstance_C|GetMapStruct (Variables|Default|GetGameInstanceRef)))) (+ (.CurrentRoom (Utilities|Struct|BreakMapGeneration (Variables|/Game/ClownsparkleContent/Blueprints/BP_GameInstance.BP_GameInstance_C|GetMapStruct (Variables|Default|GetGameInstanceRef)))) 1))))))

(event Collision|EventActorBeginOverlap
  (params (OtherActor :type Actor%20Object%20Reference)))

(event EventTick
  (params (DeltaSeconds :type Float%20%28single-precision%29)))

(fn ConstructionScript)