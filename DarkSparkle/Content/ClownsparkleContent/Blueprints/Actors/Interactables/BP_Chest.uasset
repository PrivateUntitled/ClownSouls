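; BP_Chest is a one-time interactable chest that gives the player loot or a potion when opened.
; At BeginPlay it adds a random loot drop, or, if any potion count exceeds its maximum, sometimes filters a potion list and selects Health Potion regardless.
; Interacting swings a mesh open via timeline, disables another mesh's collision, and grants harvestable-component drops, otherwise increments the potion.
; The Strength and Leaping increment branches write to each other's potion.
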(event EventBeginPlay
  (bind _gameinstanceref (Variables|Default|GetGameInstanceRef))
  (bind _gameinstanceref_2 (Variables|Default|GetGameInstanceRef))
  (bind _playerpotions (Variables|/Game/ClownsparkleContent/Blueprints/BP_GameInstance.BP_GameInstance_C|GetPlayerPotions _gameinstanceref))
  (bind _playerpotions_2 (Variables|/Game/ClownsparkleContent/Blueprints/BP_GameInstance.BP_GameInstance_C|GetPlayerPotions _gameinstanceref_2))
  (bind (_healthpotion _leapingpotion _strengthpotion) (Utilities|Struct|BreakPlayerPotions _playerpotions))
  (bind (_healthpotion_2 _leapingpotion_2 _strengthpotion_2) (Utilities|Struct|BreakPlayerPotions _playerpotions_2))
  (bind (_amount _maxamount) (Utilities|Struct|BreakHealthPotion _healthpotion))
  (bind (_amount_2 _maxamount_2) (Utilities|Struct|BreakLeapingPotion _leapingpotion_2))
  (bind (_amount_3 _maxamount_3) (Utilities|Struct|BreakStrengthPotion _strengthpotion_2))
  (bind (_amount_4 _maxamount_4) (Utilities|Struct|BreakLeapingPotion _leapingpotion))
  (bind (_amount_5 _maxamount_5) (Utilities|Struct|BreakStrengthPotion _strengthpotion))
  (bind (_amount_6 _maxamount_6) (Utilities|Struct|BreakHealthPotion _healthpotion_2))
  (|CallParentFunction)
  (bind _asbp_base_game_mode (Utilities|Casting|CastToBP_BaseGameMode (Game|GetGameMode)))
  (Variables|Default|SetNewVar _asbp_base_game_mode)
  (Collision|SetCollisionEnabled (Variables|Default|GetStaticMesh2) "QueryAndPhysics")
  (if (Math|Boolean|ORBoolean (> _amount_6 _maxamount_6) (> _amount_2 _maxamount_2) (> _amount_3 _maxamount_3))
    (if (Math|Random|RandomBoolwithWeight 0.35)
      (for _array_element (Variables|Default|GetNewVar_0)
        (switch Utilities|FlowControl|Switch|SwitchonPotions _array_element
          (:NewEnumerator0
            (if (> _amount _maxamount)
              (Utilities|Array|RemoveItem (Variables|Default|GetNewVar_0) _array_element :!label _label)))
          (:NewEnumerator1
            (if (> _amount_5 _maxamount_5)
              (goto _label)))
          (:NewEnumerator3
            (if (> _amount_4 _maxamount_4)
              (goto _label)))))
      (Variables|Default|SetPotionToAdd "NewEnumerator0")
      (else
        (Utilities|Array|Add (Variables|/Game/ClownsparkleContent/DataStorage/Components/BP_HarvestableComponent.BP_HarvestableComponent_C|GetDrops (Variables|Default|GetBP_HarvestableComponent)) (Utilities|Struct|MakeDropAmount (Utilities|Enum|ByteToEnumLoot (Math|Conversions|ToByte(Integer) (Math|Random|RandomIntegerinRange 0 (- (|GetNumEnumEntries) 1)))) (Math|Random|RandomIntegerinRange 1 3)) :!label _label_2)))
    (else
      (goto _label_2))))

(event EventOnInteract
  (bind _gameinstanceref (Variables|Default|GetGameInstanceRef))
  (bind _staticmesh1 (Variables|Default|GetStaticMesh1))
  (bind _returnvalue (Transformation|GetWorldRotation _staticmesh1))
  (bind _playerpotions (Variables|/Game/ClownsparkleContent/Blueprints/BP_GameInstance.BP_GameInstance_C|GetPlayerPotions _gameinstanceref))
  (bind (_healthpotion _leapingpotion _strengthpotion) (Utilities|Struct|BreakPlayerPotions _playerpotions))
  (bind (_roll _pitch _yaw) (Math|Rotator|BreakRotator _returnvalue))
  (if (not (Variables|Default|GetIsChestOpened))
    (Utilities|FlowControl|Sequence
      (:then_0
        (Variables|Default|SetFinalRotation (Math|Rotator|MakeRotator (- _roll 1.3e+02) _pitch _yaw))
        (bind _newtrack_0 (Timeline|Timeline Play)
          (:Update
            (Transformation|SetWorldRotation (Variables|Default|GetStaticMesh1) (Math|Rotator|Lerp(Rotator) (Transformation|GetWorldRotation (Variables|Default|GetStaticMesh1)) (Variables|Default|GetFinalRotation) _newtrack_0) false false))))
      (:then_1
        (if (!= (Utilities|Array|Length (Variables|/Game/ClownsparkleContent/DataStorage/Components/BP_HarvestableComponent.BP_HarvestableComponent_C|GetDrops (Variables|Default|GetBP_HarvestableComponent))) 0)
          (Default|AddtoPlayerLoot (Variables|Default|GetBP_HarvestableComponent))
          (else
            (switch Utilities|FlowControl|Switch|SwitchonPotions (Variables|Default|GetPotionToAdd)
              (:NewEnumerator0
                (Utilities|Struct|SetmembersinHealthPotion _healthpotion (+ (.Amount (Utilities|Struct|BreakHealthPotion _healthpotion)) 1)))
              (:NewEnumerator1
                (Utilities|Struct|SetmembersinLeapingPotion _leapingpotion (+ (.Amount (Utilities|Struct|BreakLeapingPotion _leapingpotion)) 1)))
              (:NewEnumerator3
                (Utilities|Struct|SetmembersinStrengthPotion _strengthpotion (+ (.Amount (Utilities|Struct|BreakStrengthPotion _strengthpotion)) 1))))
            (Default|CallAddLootMessage (Variables|Default|GetNewVar) (Utilities|Text|FormatText "+1 {Potion}" (Utilities|String|EnumtoString (Variables|Default|GetPotionToAdd)))))))
      (:then_2
        (Variables|Default|SetIsChestOpened true))
      (:then_3
        (Collision|SetCollisionEnabled (Variables|Default|GetStaticMesh2) "NoCollision")))))

(fn ConstructionScript
  (|CallParentFunction))