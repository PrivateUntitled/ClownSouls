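; BP_Stone is an interactable stone that the player harvests for loot.
; On OnInteract it calls AddToPlayerLoot on its BPHarvestableComponent, removes itself from the player's InteractablesInRange collection, then destroys itself.
; BeginPlay, overlap and Tick are disabled stubs, and the construction script only calls its parent.
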(event EventBeginPlay
  (|CallParentFunction) ; This node is disabled and will not be called.\nDrag off pins to build functionality.
)

(event Collision|EventActorBeginOverlap
  (params (OtherActor :type Actor%20Object%20Reference))
  (|CallParentFunction OtherActor) ; This node is disabled and will not be called.\nDrag off pins to build functionality.
)

(event EventTick
  (params (DeltaSeconds :type Float%20%28single-precision%29))
  (|CallParentFunction DeltaSeconds) ; This node is disabled and will not be called.\nDrag off pins to build functionality.
)

(event EventOnInteract
  (Default|AddtoPlayerLoot (Variables|Default|GetBP_HarvestableComponent))
  (Utilities|Array|RemoveItem (Variables|/Game/ClownsparkleContent/Blueprints/Characters/Player/BP_Player.BP_Player_C|GetInteractablesInRange (Variables|Default|GetPlayerRef)) self)
  (Actor|DestroyActor))

(fn ConstructionScript
  (|CallParentFunction))