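; Base interactable actor that tracks when the player is within reach, with an empty OnInteract event bound as the interaction hook.
; BeginPlay caches references to the player, game instance and player controller.
; Its Sphere adds the actor to the player's InteractablesInRange list on overlap.
; On end overlap, it re-queries the sphere and removes itself only if no Pawn objects still overlap.
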(event OnComponentEndOverlap(Sphere)
  (params (OverlappedComponent :type Primitive%20Component%20Object%20Reference) (OtherActor :type Actor%20Object%20Reference) (OtherComp :type Primitive%20Component%20Object%20Reference) (OtherBodyIndex :type Integer))
  (bind _self self)
  (bind _sphere (Variables|Default|GetSphere))
  (Utilities|Casting|CastToBP_Player OtherActor)
  (bind _returnvalue (Collision|ComponentOverlapActors _sphere (Transformation|GetWorldTransform _sphere) (Utilities|Array|MakeArray "ObjectTypeQuery3") 0))
  (if (not _returnvalue)
    (Utilities|IsValid _self
      (:Is%20Valid
        (Utilities|Array|RemoveItem (Variables|/Game/ClownsparkleContent/Blueprints/Characters/Player/BP_Player.BP_Player_C|GetInteractablesInRange (Variables|Default|GetPlayerRef)) _self)))))

(event OnComponentBeginOverlap(Sphere)
  (params (OverlappedComponent :type Primitive%20Component%20Object%20Reference) (OtherActor :type Actor%20Object%20Reference) (OtherComp :type Primitive%20Component%20Object%20Reference) (OtherBodyIndex :type Integer) (bFromSweep :type Boolean) (SweepResult :type Hit%20Result%20Structure%20%28by%20ref%29))
  (bind _asbp_player (Utilities|Casting|CastToBP_Player OtherActor))
  (Utilities|Array|AddUnique (Variables|/Game/ClownsparkleContent/Blueprints/Characters/Player/BP_Player.BP_Player_C|GetInteractablesInRange _asbp_player) self))

(event Custom|OnInteract)

(event EventBeginPlay
  (EventDispatchers|BindEventtoInteract (delegate Custom|OnInteract))
  (bind _asbp_player (Utilities|Casting|CastToBP_Player (Game|Player|GetPlayerPawn 0)))
  (Variables|Default|SetPlayerRef _asbp_player)
  (bind _asbp_game_instance (Utilities|Casting|CastToBP_GameInstance (Game|GetGameInstance)))
  (Variables|Default|SetGameInstanceRef _asbp_game_instance)
  (bind _asbp_player_controller (Utilities|Casting|CastToBP_PlayerController (Game|GetPlayerController 0)))
  (Variables|Default|SetPlayerControllerRef _asbp_player_controller))

(event Collision|EventActorBeginOverlap
  (params (OtherActor :type Actor%20Object%20Reference)))

(event EventTick
  (params (DeltaSeconds :type Float%20%28single-precision%29)))

(fn ConstructionScript)